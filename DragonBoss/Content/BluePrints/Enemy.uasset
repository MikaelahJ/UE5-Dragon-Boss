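; Enemy Blueprint that takes damage and hurts the player on contact.
; A handler bound to DoDamage subtracts Health behind a timed invincibility window, with death only printing a message.
; Collider overlap with Player_BP calls the player's DecreaseHealth using Strength.
; Random NavMesh wandering through AIMoveTo is present but disconnected, so it never runs.
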(event `self.ReceiveBeginPlay`
  (add `self.DoDamage` (delegate `DoDamage_Event`))
  (`KismetSystemLibrary.PrintString` (`KismetStringLibrary.Conv_IntToString` (`self.Health`))))

(event `DoDamage_Event` :!signature `self.DoDamage`
  (params (Damage :type Integer))
  (if (not (`self.Iframes`))
    (set `self.Iframes` true)
    (set `self.Health` (- (`self.Health`) Damage))
    (`KismetSystemLibrary.PrintString` (`KismetStringLibrary.Conv_IntToString` (`self.Health`)))
    (if (<= (`self.Health`) 0)
      (`KismetSystemLibrary.PrintString` "Wow good killing"))
    (`KismetSystemLibrary.Delay` (`self.IframeDuration`))
    (set `self.Iframes` false)))

(event `self.Collider.OnComponentBeginOverlap`
  (params (OverlappedComponent :type "PrimitiveComponent Object Reference") (OtherActor :type "Actor Object Reference") (OtherComp :type "PrimitiveComponent Object Reference") (OtherBodyIndex :type Integer) (bFromSweep :type Boolean) (SweepResult :type "HitResult Structure (by ref)"))
  ;[1 0 0] DoDamage
  (bind _asplayer_bp (cast `/Game/Blueprints/Player_BP` OtherActor))
  (`/Game/Blueprints/Player_BP.DecreaseHealth` _asplayer_bp (`self.Strength`)))

(fn `UserConstructionScript`)