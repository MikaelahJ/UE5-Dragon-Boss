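; HealPool_BP is a temporary healing area that restores player health over time and destroys itself 30 seconds after BeginPlay.
; A Player_BP entering the Collider sets an in-collider flag and starts a one-second Delay loop that adds clamped health and updates the HUD.
; End overlap clears the flag, which is checked after each heal, so a pending tick still lands after leaving.
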(event `self.ReceiveBeginPlay`
  (`KismetSystemLibrary.Delay` 30.0)
  (`self.K2_DestroyActor`))

(event `self.Collider.OnComponentBeginOverlap`
  (params (OverlappedComponent :type "PrimitiveComponent Object Reference") (OtherActor :type "Actor Object Reference") (OtherComp :type "PrimitiveComponent Object Reference") (OtherBodyIndex :type Integer) (bFromSweep :type Boolean) (SweepResult :type "HitResult Structure (by ref)"))
  (bind _asplayer_bp (cast `/Game/BluePrints/Player_BP` OtherActor))
  (set `self.PlayerInCollider` true)
  (`KismetSystemLibrary.Delay` 1.0 :!label _label)
  (bind _output_get (set `/Game/BluePrints/Player_BP.Health` (`KismetMathLibrary.Clamp` (+ (`/Game/BluePrints/Player_BP.Health` _asplayer_bp) 20) 0 100) _asplayer_bp))
  (`/Game/UI/HUD_Widget.UpdateHealth` (`/Game/BluePrints/Player_BP.HUD_ref` _asplayer_bp) _output_get)
  (if (`self.PlayerInCollider`)
    (goto _label)))

(event `self.Collider.OnComponentEndOverlap`
  (params (OverlappedComponent :type "PrimitiveComponent Object Reference") (OtherActor :type "Actor Object Reference") (OtherComp :type "PrimitiveComponent Object Reference") (OtherBodyIndex :type Integer))
  (cast `/Game/BluePrints/Player_BP` OtherActor)
  (set `self.PlayerInCollider` false))

(fn `UserConstructionScript`)