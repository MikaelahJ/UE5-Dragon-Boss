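; Tornado hazard Blueprint that deals repeating damage to the player character after it overlaps the tornado's collider.
; BeginPlay caches the player character, and collider overlap events set an in-range flag, with entry also starting SendDamage.
; SendDamage applies damage through a DoOnce that resets and re-enters itself after a short delay.
; The loop never checks the in-range flag, so damage continues after the player leaves.
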(event `self.ReceiveBeginPlay`
  ;[0.698 1 1] Set Player Ref
  (bind _asmy_character_bp (cast `/Game/BluePrints/MyCharacter_BP` (`GameplayStatics.GetPlayerCharacter` 0)))
  (set `self.Character Ref` _asmy_character_bp))

(event `self.Collider.OnComponentBeginOverlap`
  (params (OverlappedComponent :type "PrimitiveComponent Object Reference") (OtherActor :type "Actor Object Reference") (OtherComp :type "PrimitiveComponent Object Reference") (OtherBodyIndex :type Integer) (bFromSweep :type Boolean) (SweepResult :type "HitResult Structure (by ref)"))
  ;[1 0.2705 0.2646] See if Player is in Range
  (cast `/Game/BluePrints/MyCharacter_BP` OtherActor)
  (set `self.PlayerIsInCol` true)
  (`self.SendDamage`))

(event `self.Collider.OnComponentEndOverlap`
  (params (OverlappedComponent :type "PrimitiveComponent Object Reference") (OtherActor :type "Actor Object Reference") (OtherComp :type "PrimitiveComponent Object Reference") (OtherBodyIndex :type Integer))
  ;[1 0.2705 0.2646] See if Player is in Range
  (cast `/Game/BluePrints/MyCharacter_BP` OtherActor)
  (set `self.PlayerIsInCol` false))

(event `SendDamage`
  ;[1 0.2705 0.2646] Send Damage to Player
  (`/Engine/EditorBlueprintResources/StandardMacros.DoOnce` false :!label _label
    (:`Completed`
      (`GameplayStatics.ApplyDamage` (`self.Character Ref`) (`self.Damage`))
      (`KismetSystemLibrary.Delay` 0.4)
      (`|ExecutionSequence`
        (:`then_0`
          (goto _label :!via `Reset`))
        (:`then_1`
          (goto _label))))))

(fn `UserConstructionScript`)