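; Block actor that moves vertically when the player first enters its trigger and sets the dragon on the player.
; A one-shot overlap plays a timeline that lerps the block mesh from its current world location toward a fixed Z, applied as a relative location.
; When the timeline finishes, it disables the trigger, plays audio, tells DragonAI_BP to follow the player and plays a roar at the dragon's position.
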(event `self.Trigger.OnComponentBeginOverlap`
  (params (OverlappedComponent :type "PrimitiveComponent Object Reference") (OtherActor :type "Actor Object Reference") (OtherComp :type "PrimitiveComponent Object Reference") (OtherBodyIndex :type Integer) (bFromSweep :type Boolean) (SweepResult :type "HitResult Structure (by ref)"))
  (bind (_returnvalue_x _returnvalue_y) (`KismetMathLibrary.BreakVector` (`SceneComponent.K2_GetComponentLocation` (`self.BlockMain`))))
  (cast `/Game/BluePrints/Player_BP` OtherActor)
  (`/Engine/EditorBlueprintResources/StandardMacros.DoOnce` false
    (:`Completed`
      (bind (_direction _length) (`Timeline|Timeline` :!via `PlayFromStart`)
        (:`Update`
          (`SceneComponent.K2_SetRelativeLocation` (`self.BlockMain`) (`KismetMathLibrary.VLerp` (`SceneComponent.K2_GetComponentLocation` (`self.BlockMain`)) (`KismetMathLibrary.MakeVector` _returnvalue_x _returnvalue_y 464.0) _length) false false))
        (:`Finished`
          (`PrimitiveComponent.SetCollisionEnabled` (`self.Trigger`) "NoCollision")
          (`AudioComponent.Play` (`self.Audio`) 0.0)
          (bind _returnvalue (`GameplayStatics.GetActorOfClass` "/Game/BluePrints/DragonAI_BP.DragonAI_BP_C"))
          (`/Game/BluePrints/DragonAI_BP.FollowPlayer` _returnvalue)
          (`GameplayStatics.PlaySoundAtLocation` "/Game/Sounds/DragonRoar.DragonRoar" (`SceneComponent.K2_GetComponentLocation` (`/Game/BluePrints/DragonAI_BP.BodyCollider` _returnvalue)) (struct) 1.0 1.0 0.0 null null null null))))))

(fn `UserConstructionScript`)