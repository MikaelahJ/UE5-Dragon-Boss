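; Spawner actor that periodically places HealPool_BP actors at random points within its own bounds.
; BeginPlay caches the Player_BP character, stopping if the cast fails, then waits before starting SpawnHeal.
; SpawnHeal re-calls itself after a delay, looping indefinitely.
; A SpawnBall event uses the same random-point spawn, but has no class set and is not called within this Blueprint.
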(event `self.ReceiveBeginPlay`
  ;[0.3397 1 0.9302] Begin Spawning
  (bind _asplayer_bp (cast `/Game/BluePrints/Player_BP` (`GameplayStatics.GetPlayerCharacter` 0)))
  (set `self.Player` _asplayer_bp)
  (`KismetSystemLibrary.Delay` 10.0)
  (`self.SpawnHeal`))

(event `SpawnHeal`
  (bind (_origin _boxextent) (`self.GetActorBounds` false))
  ;[0.09375 1 0.1766] Spawn HealPool
  (`|SpawnActorFromClass` "/Game/BluePrints/HealPool_BP.HealPool_BP_C" (`KismetMathLibrary.MakeTransform` (`KismetMathLibrary.RandomPointInBoundingBox` _origin _boxextent)) "AdjustIfPossibleButAlwaysSpawn" "OverrideRootScale" null null)
  (`KismetSystemLibrary.Delay` 10.0)
  (`self.SpawnHeal`))

(event `SpawnBall`
  (bind (_origin _boxextent) (`self.GetActorBounds` false))
  ;[1 0.1063 0.09896] Spawn Ball
  (`|SpawnActorFromClass` "/Game/BluePrints/HittableBall_BP.HittableBall_BP_C" (`KismetMathLibrary.MakeTransform` (`KismetMathLibrary.RandomPointInBoundingBox` _origin _boxextent)) "AdjustIfPossibleButAlwaysSpawn" "OverrideRootScale" null null))

(fn `UserConstructionScript`)