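; AmmoSpawner_BP is an actor that spawns ammo boxes at random points in the level.
; On BeginPlay it stores three target point references in an array.
; Its SpawnAmmo event picks one at random and spawns an AmmoBox_BP at that transform, adjusting for collisions but always spawning.
; Nothing in this Blueprint calls SpawnAmmo, so the event relies on an external trigger.
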(event `self.ReceiveBeginPlay`
  ;[1 1 1] Create array of targetpoints
  (set `self.AmmoArray` (`|MakeArray` (`self.AmmoTarget1`) (`self.AmmoTarget2`) (`self.AmmoTarget3`))))

(event `SpawnAmmo`
  ;[1 1 1] Event to spawn ammobox on random targetpoint from array
  (`|SpawnActorFromClass` "/Game/BluePrints/AmmoBox_BP.AmmoBox_BP_C" (`self.GetTransform` (`|GetArrayItem` (`self.AmmoArray`) (`KismetMathLibrary.RandomIntegerInRange` 0 2))) "AdjustIfPossibleButAlwaysSpawn" "OverrideRootScale" null null))

(fn `UserConstructionScript`)