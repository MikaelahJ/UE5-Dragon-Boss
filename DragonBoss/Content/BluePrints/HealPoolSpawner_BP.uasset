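; HealPoolSpawner_BP is an actor that periodically spawns HealPool_BP actors at random points within its own bounds.
; On BeginPlay it caches the player as MyCharacter_BP, stopping if the cast fails, then waits before the first spawn.
; SpawnHeal picks a point in the actor's bounding box, spawns with collision adjustment, then re-calls itself after a Delay, looping indefinitely without limiting the pool count.
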(event `self.ReceiveBeginPlay`
  (bind _asmy_character_bp (cast `/Game/BluePrints/MyCharacter_BP` (`GameplayStatics.GetPlayerCharacter` 0)))
  (set `self.Player` _asmy_character_bp)
  (`KismetSystemLibrary.Delay` 10.0)
  (`self.SpawnHeal`))

(event `SpawnHeal`
  (bind (_origin _boxextent) (`self.GetActorBounds` false))
  (`|SpawnActorFromClass` "/Game/BluePrints/HealPool_BP.HealPool_BP_C" (`KismetMathLibrary.MakeTransform` (`KismetMathLibrary.RandomPointInBoundingBox` _origin _boxextent)) "AdjustIfPossibleButAlwaysSpawn" "OverrideRootScale" null null)
  (`KismetSystemLibrary.Delay` 15.0)
  (`self.SpawnHeal`))

(fn `UserConstructionScript`)