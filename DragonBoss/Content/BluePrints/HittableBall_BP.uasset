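; HittableBall_BP is a ball projectile that can be sent at the dragon to damage it.
; SendToDragon makes it home on the dragon's body collider, ignores the player when moving and arms it to deal damage.
; Overlapping that collider while armed stops the ball, swaps in a water-ball hit particle and damages the dragon once.
; After a short delay it tells Spawner_BP to spawn a ball, then destroys itself.
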(event `self.ReceiveBeginPlay`
  ;[0.698 1 1] Get references
  (bind _asplayer_bp (cast `/Game/BluePrints/Player_BP` (`GameplayStatics.GetPlayerCharacter` 0)))
  (set `self.Player_ref` _asplayer_bp)
  (bind _returnvalue (`GameplayStatics.GetActorOfClass` "/Game/BluePrints/DragonAI_BP.DragonAI_BP_C"))
  (set `self.Dragon_ref` _returnvalue))

(event `SendToDragon`
  (bind _projectilemovement (`self.ProjectileMovement`))
  ;[1 0.9216 0.3663] Set Dragoon as homing target
  (set `ProjectileMovementComponent.bIsHomingProjectile` true _projectilemovement)
  (set `ProjectileMovementComponent.HomingTargetComponent` (`/Game/BluePrints/DragonAI_BP.BodyCollider` (`self.Dragon_ref`)) _projectilemovement)
  (`PrimitiveComponent.IgnoreActorWhenMoving` (`self.Collider`) (`self.Player_ref`) true)
  (set `self.CanHitDragon` true))

(event `self.Collider.OnComponentBeginOverlap`
  (params (OverlappedComponent :type "PrimitiveComponent Object Reference") (OtherActor :type "Actor Object Reference") (OtherComp :type "PrimitiveComponent Object Reference") (OtherBodyIndex :type Integer) (bFromSweep :type Boolean) (SweepResult :type "HitResult Structure (by ref)"))
  ;[1 0.2705 0.2646] If Hit Dragon
  (bind _asdragon_ai_bp (cast `/Game/BluePrints/DragonAI_BP` OtherActor))
  (if (== (`/Game/BluePrints/DragonAI_BP.BodyCollider` _asdragon_ai_bp) OtherComp)
    (if (`self.CanHitDragon`)
      (`MovementComponent.StopMovementImmediately` (`self.ProjectileMovement`))
      (`ParticleSystemComponent.SetTemplate` (`self.ParticleSystem`) "/Game/FXVarietyPack/Particles/P_ky_waterBallHit.P_ky_waterBallHit")
      (`/Game/BluePrints/DragonAI_BP.TakeDamage` (`self.Dragon_ref`) (`self.Damage`))
      (set `self.CanHitDragon` false)
      (`KismetSystemLibrary.Delay` 0.5)
      (bind _returnvalue (`GameplayStatics.GetActorOfClass` "/Game/BluePrints/Spawner_BP.Spawner_BP_C"))
      (`/Game/BluePrints/Spawner_BP.SpawnBall` _returnvalue)
      (`self.K2_DestroyActor`))))

(fn `UserConstructionScript`)